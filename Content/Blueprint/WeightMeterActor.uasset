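; Weight meter actor that turns BalanceBoard readings into an on-screen scale display.
; BeginPlay creates the UI-only widget, spawns a MeterKG2 dial and collects the level's BalanceBar actors by index.
; A Delay on Tick throttles polling to about 30 Hz, and board state changes show Japanese status messages.
; Lerp-smoothed, non-negative weight drives the readout and dial roll, while the four sensor values scale the bars in X and Y.
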(event Custom|L_SetStateMessage
  (params (NewState :type EBalanceBoardState%20Enum))
  (if (Utilities|Enum|NotEqual(Enum) (Variables|UMG|GetPrevState) NewState)
    (bind _output_get (Variables|UMG|SetPrevState NewState))
    (switch Utilities|FlowControl|Switch|SwitchonEBalanceBoardState _output_get
      (:STATE_BUSY
        (CallFunction|SetMeterMessage "初期化しています。しばらくお待ちください。"))
      (:STATE_DEVICE_NOT_FOUND
        (CallFunction|SetMeterMessage "BalanceBoard が見つかりません。”Add Device\" ボタンを押してください。"))
      (:STATE_CALIBRATION
        (CallFunction|SetMeterMessage "０Kg  調整中です。"))
      (:STATE_READY
        (CallFunction|SetMeterMessage))
      (:STATE_ADD_DEVICE
        (CallFunction|SetMeterMessage "登録します。BalanceBoard の Sync ボタンを押してしばらくお待ちください。"))
      (:STATE_WAIT_DEVICE
        (CallFunction|SetMeterMessage "情報を取得しています。しばらくお待ちください。")))))

(event EventTick
  (params (DeltaSeconds :type Float%20%28single-precision%29))
  (bind _balancedata (Variables|Balance|GetBalanceData))
  (Utilities|FlowControl|Delay 0.0333)
  (bind (_weight _w0 _w1 _w2 _w3 _state _returnvalue) (Class|BalanceBoardFunction|UpdateBalanceBoard))
  (CallFunction|LSetStateMessage _state)
  (if _returnvalue
    (Utilities|Array|SetArrayElem _balancedata 0 _w0)
    (Utilities|Array|SetArrayElem _balancedata 1 _w1)
    (Utilities|Array|SetArrayElem _balancedata 2 _w2)
    (Utilities|Array|SetArrayElem _balancedata 3 _w3)
    (bind _weight_2 (CallFunction|GetWeightValue _weight))
    (CallFunction|SetMeterValue _weight_2)
    (Transformation|SetActorRotation (Variables|Default|GetMeterKG_Ref) (Math|Rotator|MakeRotator (- (* _weight_2 2.0) 1.2e+02) 0.0 0.0) true)
    (for (_array_element _array_index) (Variables|Balance|GetBalanceBar_Ref)
      (Transformation|SetActorScale3D _array_element (Math|Vector|MakeVector (+ (* (Utilities|Array|Get(acopy) (Variables|Balance|GetBalanceData) _array_index) 0.07) 0.1) (+ (* (Utilities|Array|Get(acopy) (Variables|Balance|GetBalanceData) _array_index) 0.07) 0.1) 1.0)))))

(event EventBeginPlay
  (bind _returnvalue (Game|GetPlayerController 0))
  (bind _returnvalue_2 (Transformation|GetActorTransform))
  (bind _returnvalue_3 (UserInterface|CreateWidget "/Game/UMG/WeightMeterWidget.WeightMeterWidget_C" (Game|GetPlayerController 0)))
  (bind _output_get (Variables|UMG|SetWeightMeterWidget_Ref _returnvalue_3))
  (UserInterface|Viewport|AddtoViewport _output_get 0)
  (Input|SetInputModeUIOnly _returnvalue 0 false)
  (Variables|/Script/Engine.PlayerController|SetbShowMouseCursor _returnvalue true)
  (bind _returnvalue_4 (Game|SpawnActorfromClass "/Game/Blueprint/MeterKG2.MeterKG2_C" (Math|Transform|MakeTransform (+ (.location _returnvalue_2) "0, 0,50.000000") (.rotation _returnvalue_2) (.scale _returnvalue_2)) "Undefined" 0 0))
  (Variables|Default|SetMeterKG_Ref _returnvalue_4)
  (Utilities|Array|Resize (Variables|Balance|GetBalanceData) 4)
  (Utilities|Array|Resize (Variables|Balance|GetBalanceBar_Ref) 4)
  (bind _outactors (Actor|GetAllActorsOfClass "/Game/Blueprint/BalanceBar.BalanceBar_C"))
  (for _array_element _outactors
    (Utilities|Array|SetArrayElem (Variables|Balance|GetBalanceBar_Ref) (Variables|/Game/Blueprint/BalanceBar.BalanceBar_C|GetIndex _array_element) _array_element true)))

(fn ConstructionScript)

(fn SetMeterMessage
  (params (Text :type Text))
  (Rendering|Components|TextRender|SetText (Variables|/Game/UMG/WeightMeterWidget.WeightMeterWidget_C|GetMessage (Variables|UMG|GetWeightMeterWidget_Ref)) Text))

(fn GetWeightValue
  (params (Value :type Float%20%28single-precision%29))
  (bind _output_get (Variables|UMG|SetPrevWeight (Math|Float|Lerp (Variables|UMG|GetPrevWeight) (Math|Float|Max(Float) Value 0.0) 0.5)))
  (return _output_get))

(fn SetMeterValue
  (params (Value :type Float%20%28single-precision%29))
  (Rendering|Components|TextRender|SetText (Variables|/Game/UMG/WeightMeterWidget.WeightMeterWidget_C|GetWeightValue (Variables|UMG|GetWeightMeterWidget_Ref)) (Utilities|Text|ToText(Float) Value "HalfToEven" true 1 324 0 1)))